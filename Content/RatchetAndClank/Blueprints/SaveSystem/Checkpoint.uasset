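; Checkpoint trigger actor that saves the game at its own location and rotation when Ratchet enters its collision box.
; A short delay after BeginPlay arms saving, then an overlap by Ratchet calls SaveAll with the checkpoint flag and destroys the actor, making it single-use.
; The construction script scales the Cube mesh from the collision box's extent.
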(event OnComponentBeginOverlap(Collision)
  (params (OverlappedComponent :type Primitive%20Component%20Object%20Reference) (OtherActor :type Actor%20Object%20Reference) (OtherComp :type Primitive%20Component%20Object%20Reference) (OtherBodyIndex :type Integer) (bFromSweep :type Boolean) (SweepResult :type Hit%20Result%20Structure%20%28by%20ref%29))
  (bind _returnvalue (Transformation|GetActorTransform))
  (if (Variables|Default|GetCanSave)
    (bind _asratchet (Utilities|Casting|CastToRatchet OtherActor))
    (Default|SaveAll _asratchet (Math|Transform|MakeTransform (.location _returnvalue) (.rotation _returnvalue) "1,1,1") true)
    (Variables|Default|SetCanSave true)
    (Actor|DestroyActor)))

(event EventBeginPlay
  (Utilities|FlowControl|Delay 2.0)
  (Variables|Default|SetCanSave true))

(fn ConstructionScript
  (bind _collision (Variables|Default|GetCollision))
  (bind _boxextent (Variables|/Script/Engine.BoxComponent|GetBoxExtent _collision))
  (Transformation|SetWorldScale3D (Variables|Default|GetCube) (Math|Vector|MakeVector (/ (.x _boxextent) 25.0) (/ (.y _boxextent) 25.0) (/ (.z _boxextent) 25.0))))
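; Base weapon Blueprint for a Ratchet & Clank game, with empty fire, alt-fire, wrench and level-up events, presumably for child weapons.
; Ammo pickups clamp to the maximum and refresh the player's HUD; XP levels the weapon at level-scaled thresholds until max level.
; Ammo, level and XP persist in a save slot keyed by weapon name, loaded on BeginPlay.
; A helper computes two points on a ballistic arc.
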(event Custom|Alt%20Fire%20Released
  ;[1 1 1] Weapon Atributes
)

(event Custom|Wrench
  ;[1 1 1] Weapon Atributes
)

(event Custom|Level%20Up
  ;[1 1 1] Weapon Atributes
)

(event Custom|UpdateMainUIWithAmmo
  ;[1 1 1] Weapon Atributes
  (bind _asratchet (Utilities|Casting|CastToRatchet (Game|Player|GetPlayerPawn 0)))
  (if (Utilities|IsValid (Variables|/Game/RatchetAndClank/Blueprints/Actors/Characters/Pawns/Ratchet.Ratchet_C|GetGamePlayUIWidget _asratchet))
    (Default|UpdateGunAmmo (Variables|/Game/RatchetAndClank/Blueprints/Actors/Characters/Pawns/Ratchet.Ratchet_C|GetGamePlayUIWidget _asratchet))))

(event Custom|Fire%20Pressed
  ;[1 1 1] Weapon Atributes
)

(event Custom|Experience%20Get
  (params (XP :type Float%20%28single-precision%29))
  ;[1 1 1] Weapon Atributes
  (Variables|Statistics|SetXP (+ (Variables|Statistics|GetXP) XP))
  (if (and (!= (Variables|Statistics|GetLevel) (Variables|Statistics|GetMaxLevel)) (>= (Variables|Statistics|GetXP) (* (Variables|Statistics|GetLevel) 1e+03)))
    (Variables|Statistics|SetXP 0.0)
    (Math|Integer|IncrementInt (Variables|Statistics|GetLevel)
      (:%20%20
        (CallFunction|UpdateMainUIwithAmmo)
        (CallFunction|LevelUp)))))

(event Custom|Alt%20Fire%20Pressed
  ;[1 1 1] Weapon Atributes
)

(event Custom|Ammo%20Get
  (params (Amount :type Integer))
  ;[1 1 1] Weapon Atributes
  (Variables|Statistics|SetAmmo (Math|Integer|Clamp(Integer) (+ Amount (Variables|Statistics|GetAmmo)) 0 (Variables|Statistics|GetMaxAmmo)))
  (CallFunction|UpdateMainUIwithAmmo))

(event Custom|Save
  ;[1 1 1] Weapon Atributes
  (bind _returnvalue (SaveGame|CreateSaveGameObject "/Game/RatchetAndClank/Blueprints/SaveSystem/WeaponSave.WeaponSave_C"))
  (bind _asweapon_save (Utilities|Casting|CastToWeaponSave _returnvalue))
  (bind _output_get (Variables|Accesories|SetWeaponSaveInstance _asweapon_save))
  (Variables|/Game/RatchetAndClank/Blueprints/SaveSystem/WeaponSave.WeaponSave_C|SetAmmo _output_get (Variables|Statistics|GetAmmo))
  (Variables|/Game/RatchetAndClank/Blueprints/SaveSystem/WeaponSave.WeaponSave_C|SetLevel _output_get (Variables|Statistics|GetLevel))
  (Variables|/Game/RatchetAndClank/Blueprints/SaveSystem/WeaponSave.WeaponSave_C|SetXP _output_get (Variables|Statistics|GetXP))
  (SaveGame|SaveGametoSlot (Variables|Accesories|GetWeaponSaveInstance) (Variables|Statistics|GetWeaponName))
  (Development|PrintString "SavedWeapons"))

(event Custom|Fire%20Released
  ;[1 1 1] Weapon Atributes
)

(event EventBeginPlay
  (Utilities|FlowControl|Sequence
    (:then_0
      (bind _returnvalue (SaveGame|DoesSaveGameExist (Variables|Statistics|GetWeaponName)))
      (if _returnvalue
        (bind _returnvalue_2 (SaveGame|LoadGamefromSlot (Variables|Statistics|GetWeaponName)))
        (bind _asweapon_save (Utilities|Casting|CastToWeaponSave _returnvalue_2))
        (bind _output_get (Variables|Accesories|SetWeaponSaveInstance _asweapon_save))
        (Variables|Statistics|SetAmmo (Variables|/Game/RatchetAndClank/Blueprints/SaveSystem/WeaponSave.WeaponSave_C|GetAmmo _output_get))
        (Variables|Statistics|SetLevel (Variables|/Game/RatchetAndClank/Blueprints/SaveSystem/WeaponSave.WeaponSave_C|GetLevel _output_get))
        (Variables|Statistics|SetXP (Variables|/Game/RatchetAndClank/Blueprints/SaveSystem/WeaponSave.WeaponSave_C|GetXP _output_get))
        (CallFunction|UpdateMainUIwithAmmo)
        (else
          (Variables|Statistics|SetAmmo (Variables|Statistics|GetMaxAmmo)))))))

(fn ConstructionScript)

(fn GetSegments0
  (params (Start%20Location :type Vector) (Initial%20Velocity :type Vector) (Gravity :type Vector) (Time1 :type Float%20%28single-precision%29) (Time2 :type Float%20%28single-precision%29))
  (return (+ Start%20Location (* Initial%20Velocity Time1) (* Gravity (* Time1 Time1 0.5))) (+ Start%20Location (* Initial%20Velocity Time2) (* Gravity (* Time2 Time2 0.5)))))
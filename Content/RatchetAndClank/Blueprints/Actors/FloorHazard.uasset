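; FloorHazard is a timed floor trap that periodically emits a damaging effect.
; After an initial Offset delay, Emit re-calls itself in an endless loop, holding the particle effect, box collision and point light on for TimeEnabled, then off for TimeDisabled.
; While active, any actor that begins overlapping the box takes FireAndLava damage.
; The effect template comes from the Effect variable, applied at BeginPlay.
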(event OnComponentBeginOverlap(Box)
  (params (OverlappedComponent :type Primitive%20Component%20Object%20Reference) (OtherActor :type Actor%20Object%20Reference) (OtherComp :type Primitive%20Component%20Object%20Reference) (OtherBodyIndex :type Integer) (bFromSweep :type Boolean) (SweepResult :type Hit%20Result%20Structure%20%28by%20ref%29))
  (Game|Damage|ApplyDamage OtherActor 1.0 0 0 "/Game/RatchetAndClank/Blueprints/DamageTypes/FireAndLava.FireAndLava_C"))

(event Custom|Emit
  (bind _pointlight (Variables|Default|GetPointLight))
  (bind _particlesystem (Variables|Default|GetParticleSystem))
  (bind _box (Variables|Default|GetBox))
  (Components|Activation|Activate _particlesystem false)
  (Collision|SetCollisionEnabled _box "QueryOnly")
  (Rendering|Components|Light|SetIntensity _pointlight 1e+05)
  (Utilities|FlowControl|Delay (Variables|Default|GetTimeEnabled))
  (Components|Activation|Deactivate _particlesystem)
  (Collision|SetCollisionEnabled _box "NoCollision")
  (Rendering|Components|Light|SetIntensity _pointlight 0.0)
  (Utilities|FlowControl|Delay (Variables|Default|GetTimeDisabled))
  (CallFunction|Emit))

(event EventBeginPlay
  (Effects|Components|ParticleSystem|SetTemplate (Variables|Default|GetParticleSystem) (Variables|Default|GetEffect))
  (Utilities|FlowControl|Delay (Variables|Default|GetOffset))
  (CallFunction|Emit))

(event Collision|EventActorBeginOverlap
  (params (OtherActor :type Actor%20Object%20Reference)))

(event EventTick
  (params (DeltaSeconds :type Float%20%28single-precision%29)))

(fn ConstructionScript)
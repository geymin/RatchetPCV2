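; Spline path actor that flies a set of registered ships in a continuous loop at a shared speed.
; AddNewShip collects ships, using a tiny retriggerable delay to batch calls before spacing them evenly along the spline and recording their distances.
; Tick advances each valid ship's distance by ShipSpeed, wraps it past the spline's end, and sets its root location and rotation from the spline.
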(event Custom|AddNewShip
  (params (newShip :type Breakable%20Ship%20Base%20Object%20Reference))
  (bind _ships (Variables|Default|Getships))
  (bind _spline (Variables|Default|GetSpline))
  (bind _returnvalue (Utilities|Array|Length _ships))
  (Utilities|Array|Add _ships newShip)
  (Utilities|FlowControl|RetriggerableDelay 0.001)
  (for (_array_element _array_index) _ships
    (Transformation|SetWorldLocation (Variables|/Game/RatchetAndClank/Blueprints/Actors/Breakables/BaseBreakable.BaseBreakable_C|GetDefaultSceneRoot _array_element) (Spline|GetLocationatDistanceAlongSpline _spline (* _array_index (/ (Spline|GetSplineLength (Variables|Default|GetSpline)) (Math|Conversions|ToFloat(Integer) _returnvalue))) "World") false false)
    (Transformation|SetWorldRotation (Variables|/Game/RatchetAndClank/Blueprints/Actors/Breakables/BaseBreakable.BaseBreakable_C|GetDefaultSceneRoot _array_element) (Spline|GetRotationatDistanceAlongSpline _spline (* _array_index (/ (Spline|GetSplineLength (Variables|Default|GetSpline)) (Math|Conversions|ToFloat(Integer) _returnvalue))) "World") false false)
    (Utilities|Array|Add (Variables|Default|GetshipPositionsOnSpline) (* _array_index (/ (Spline|GetSplineLength (Variables|Default|GetSpline)) (Math|Conversions|ToFloat(Integer) _returnvalue)))))
  (Variables|Default|SetshipsOnSpline _returnvalue))

(event EventBeginPlay)

(event Collision|EventActorBeginOverlap
  (params (OtherActor :type Actor%20Object%20Reference)))

(event EventTick
  (params (DeltaSeconds :type Float%20%28single-precision%29))
  (bind _shippositionsonspline (Variables|Default|GetshipPositionsOnSpline))
  (bind _spline (Variables|Default|GetSpline))
  (bind _returnvalue (Spline|GetSplineLength _spline))
  (for (_array_element _array_index) (Variables|Default|Getships)
    (Utilities|IsValid _array_element
      (:Is%20Valid
        (if (> (+ (Utilities|Array|Get(acopy) _shippositionsonspline _array_index) (* (Variables|Default|GetshipSpeed) DeltaSeconds)) _returnvalue)
          (Utilities|Array|SetArrayElem _shippositionsonspline _array_index (- (+ (Utilities|Array|Get(acopy) _shippositionsonspline _array_index) (* (Variables|Default|GetshipSpeed) DeltaSeconds)) _returnvalue))
          (Transformation|SetWorldLocation (Variables|/Game/RatchetAndClank/Blueprints/Actors/Breakables/BaseBreakable.BaseBreakable_C|GetDefaultSceneRoot _array_element) (Spline|GetLocationatDistanceAlongSpline _spline (- (+ (Utilities|Array|Get(acopy) _shippositionsonspline _array_index) (* (Variables|Default|GetshipSpeed) DeltaSeconds)) _returnvalue) "World") false false)
          (Transformation|SetWorldRotation (Variables|/Game/RatchetAndClank/Blueprints/Actors/Breakables/BaseBreakable.BaseBreakable_C|GetDefaultSceneRoot _array_element) (Spline|GetRotationatDistanceAlongSpline _spline (- (+ (Utilities|Array|Get(acopy) _shippositionsonspline _array_index) (* (Variables|Default|GetshipSpeed) DeltaSeconds)) _returnvalue) "Local") false false)
          (else
            (Utilities|Array|SetArrayElem _shippositionsonspline _array_index (+ (Utilities|Array|Get(acopy) _shippositionsonspline _array_index) (* (Variables|Default|GetshipSpeed) DeltaSeconds)))
            (Transformation|SetWorldLocation (Variables|/Game/RatchetAndClank/Blueprints/Actors/Breakables/BaseBreakable.BaseBreakable_C|GetDefaultSceneRoot _array_element) (Spline|GetLocationatDistanceAlongSpline _spline (+ (Utilities|Array|Get(acopy) _shippositionsonspline _array_index) (* (Variables|Default|GetshipSpeed) DeltaSeconds)) "World") false false)
            (Transformation|SetWorldRotation (Variables|/Game/RatchetAndClank/Blueprints/Actors/Breakables/BaseBreakable.BaseBreakable_C|GetDefaultSceneRoot _array_element) (Spline|GetRotationatDistanceAlongSpline _spline (+ (Utilities|Array|Get(acopy) _shippositionsonspline _array_index) (* (Variables|Default|GetshipSpeed) DeltaSeconds)) "Local") false false)))))))

(fn ConstructionScript)
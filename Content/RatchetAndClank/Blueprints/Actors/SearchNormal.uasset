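; SearchNormal is a debug actor that reports surface normals on either side of itself.
; On BeginPlay it caches the player's Ratchet character so traces can ignore it.
; Each Tick it fires long Visibility line traces along its negative and positive right vector, drawn for one frame.
; Each hit normal is printed on screen in its own color, blue for one side and yellow for the other.
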(event EventTick
  (params (DeltaSeconds :type Float%20%28single-precision%29))
  (bind _returnvalue (Transformation|GetActorLocation))
  (bind _returnvalue_2 (Transformation|GetActorLocation))
  (bind _ratchet (Variables|Default|GetRatchet))
  (bind _array (Utilities|Array|MakeArray _ratchet))
  (Utilities|FlowControl|Sequence
    (:then_0
      (bind _outhit (Collision|LineTraceByChannel _returnvalue_2 (+ _returnvalue_2 (* (Transformation|GetActorRightVector) -5e+04)) "TraceTypeQuery1" false _array "ForOneFrame"))
      (Development|PrintString (Utilities|String|ToString(Vector) (.normal _outhit)) true true "(R=0.214241,G=0.000000,B=1.000000,A=1.000000)"))
    (:then_1
      (bind _outhit_2 (Collision|LineTraceByChannel _returnvalue (+ _returnvalue (* (Transformation|GetActorRightVector) 5e+04)) "TraceTypeQuery1" false _array "ForOneFrame"))
      (Development|PrintString (Utilities|String|ToString(Vector) (.normal _outhit_2)) true true "(R=0.889259,G=1.000000,B=0.000000,A=1.000000)"))))

(event EventBeginPlay
  (bind _asratchet (Utilities|Casting|CastToRatchet (Game|GetPlayerCharacter 0)))
  (Variables|Default|SetRatchet _asratchet))

(fn ConstructionScript)
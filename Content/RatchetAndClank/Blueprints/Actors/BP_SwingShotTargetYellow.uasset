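; Yellow Swing Shot target actor that keeps turning to face Ratchet.
; Each tick it sets the root sphere's yaw from a look-at rotation toward Ratchet, keeping pitch and roll at zero.
; The construction script sizes a sphere radius and a second scaled sphere from DistanceLimit, so both match the range, then runs the parent's construction script.
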(event EventTick
  (params (DeltaSeconds :type Float%20%28single-precision%29))
  (Transformation|SetWorldRotation (Variables|Default|GetRootSphere) (Math|Rotator|MakeRotator 0.0 0.0 (.yaw (Math|Rotator|FindLookatRotation (Transformation|GetActorLocation) (Transformation|GetActorLocation (Variables|Default|GetRatchet))))) false false))

(fn ConstructionScript
  (bind _distancelimit (Variables|Default|GetDistanceLimit))
  (bind _returnvalue (/ _distancelimit 5e+01))
  (Components|Sphere|SetSphereRadius (Variables|Default|GetSphere) _distancelimit true)
  (Transformation|SetWorldScale3D (Variables|Default|GetSphere1) (Math|Vector|MakeVector _returnvalue _returnvalue _returnvalue))
  (|CallParentFunction))
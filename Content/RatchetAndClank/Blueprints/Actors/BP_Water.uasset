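; Water volume for the Ratchet character that switches the player into surface swimming, or sets walk-on-water when not swimmable.
; Box overlap starts swimming: movement is slowed, the weapon hidden, and a buoyancy timeline settles Ratchet just below the plane.
; Events handle diving with flying movement and exiting the water.
; Tick compares heights with the water plane to resurface a diving Ratchet and toggle a runtime-added post process while the camera is submerged.
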(event OnComponentBeginOverlap(Box)
  (params (OverlappedComponent :type Primitive%20Component%20Object%20Reference) (OtherActor :type Actor%20Object%20Reference) (OtherComp :type Primitive%20Component%20Object%20Reference) (OtherBodyIndex :type Integer) (bFromSweep :type Boolean) (SweepResult :type Hit%20Result%20Structure%20%28by%20ref%29))
  (bind _ratchet (Variables|Default|GetRatchet))
  (bind _ratchet_2 (Variables|Default|GetRatchet))
  (bind _ratchet_3 (Variables|Default|GetRatchet))
  (bind _returnvalue (Transformation|GetActorLocation _ratchet_3))
  (bind _charactermovement (Variables|/Script/Engine.Character|GetCharacterMovement _ratchet_3))
  (bind _charactermovement_2 (Variables|/Script/Engine.Character|GetCharacterMovement _ratchet))
  (bind _wrench (Variables|/Game/RatchetAndClank/Blueprints/Actors/Characters/Pawns/Ratchet.Ratchet_C|GetWrench _ratchet))
  (if (and (== OtherActor _ratchet_2) (not (Variables|/Game/RatchetAndClank/Blueprints/Actors/Characters/Pawns/Ratchet.Ratchet_C|GetJump%20Ledge _ratchet_2)))
    (if (Variables|Default|GetIs%20Swimmable?)
      (CallFunction|IsNowSwimmable)
      (Utilities|FlowControl|Sequence
        (:then_0
          (Variables|/Game/RatchetAndClank/Blueprints/Actors/Characters/Pawns/Ratchet.Ratchet_C|SetWaterPLane _ratchet_2 self)
          (Rendering|SetActorHiddenInGame (Variables|/Game/RatchetAndClank/Blueprints/Actors/Characters/Pawns/Ratchet.Ratchet_C|GetCurrentWeapon _ratchet_2) true)
          (Variables|/Script/Engine.CharacterMovementComponent|SetMaxFlySpeed (Variables|/Script/Engine.Character|GetCharacterMovement _ratchet_2) 2e+02)
          (Variables|/Game/RatchetAndClank/Blueprints/Actors/Characters/Pawns/Ratchet.Ratchet_C|SetShouldSetCameraZ _ratchet_3 false)
          (Utilities|FlowControl|Sequence
            (:then_0
              (Variables|/Game/RatchetAndClank/Blueprints/Actors/Characters/Pawns/Ratchet.Ratchet_C|SetJumpedOnWater _ratchet_3 false)
              (Class|MovementComponent|SetPlaneConstraintEnabled (Variables|/Script/Engine.Character|GetCharacterMovement _ratchet_3) true)
              (Variables|/Game/RatchetAndClank/Blueprints/Actors/Characters/Pawns/Ratchet.Ratchet_C|SetSwimming _ratchet_3 true)
              (Variables|/Game/RatchetAndClank/Blueprints/Actors/Characters/Pawns/Ratchet.Ratchet_C|SetSwimmingStates _ratchet_3 "NewEnumerator1")
              (Variables|/Script/Engine.CharacterMovementComponent|SetMaxWalkSpeed _charactermovement 2e+02)
              (Variables|/Script/Engine.CharacterMovementComponent|SetBrakingDecelerationFalling _charactermovement 2e+02)
              (Variables|/Script/Engine.CharacterMovementComponent|SetFallingLateralFriction _charactermovement 1.0)
              (Default|ExitLedge _ratchet)
              (Variables|/Game/RatchetAndClank/Blueprints/Actors/Inventory/Weapons/OmniWrench.OmniWrench_C|SetDamage1 _wrench false)
              (Variables|/Game/RatchetAndClank/Blueprints/Actors/Inventory/Weapons/OmniWrench.OmniWrench_C|SetDamage2 _wrench false)
              (Variables|/Game/RatchetAndClank/Blueprints/Actors/Inventory/Weapons/OmniWrench.OmniWrench_C|SetDamage3 _wrench false)
              (Variables|/Game/RatchetAndClank/Blueprints/Actors/Inventory/Weapons/OmniWrench.OmniWrench_C|SetHypDamage _wrench false)
              (Audio|PlaySoundatLocation "/Game/RatchetAndClank/Sounds/SFX/RC1Sfx/EnterWater_Cue.EnterWater_Cue" (Transformation|GetActorLocation (Variables|Default|GetRatchet)) "0, 0, 0" 1.0 1.0 0.0 0 0 0)
              (Variables|/Script/Engine.MovementComponent|SetVelocity _charactermovement_2 (/ (Variables|/Script/Engine.MovementComponent|GetVelocity _charactermovement_2) 3.0))
              (bind _returnvalue_2 (AddComponent|AddPostProcessComponent false))
              (bind _output_get (Variables|Default|Setpost _returnvalue_2))
              (Variables|/Script/Engine.PostProcessComponent|SetbEnabled _output_get false))
            (:then_1
              (|NOde _ratchet_3))))
        (:then_1
          (Variables|/Game/RatchetAndClank/Blueprints/Actors/Characters/Pawns/Ratchet.Ratchet_C|SetCan't%20Move _ratchet_3 true)
          (bind _newtrack_0 (Timeline|Bouyancy PlayFromStart)
            (:Update
              (Transformation|SetActorLocation _ratchet_3 (Math|Vector|MakeVector (.x _returnvalue) (.y _returnvalue) (+ _newtrack_0 (.z _returnvalue))) false false))
            (:Finished
              (Transformation|SetActorLocation _ratchet_3 (Math|Vector|MakeVector (.x _returnvalue) (.y _returnvalue) (+ (.z (Transformation|GetActorLocation (Variables|/Game/RatchetAndClank/Blueprints/Actors/Characters/Pawns/Ratchet.Ratchet_C|GetWaterPLane _ratchet_2))) -2e+01)) false false)))))
      (else
        (CallFunction|IsNotSwimmable)))))

(event OnComponentEndOverlap(Box)
  (params (OverlappedComponent :type Primitive%20Component%20Object%20Reference) (OtherActor :type Actor%20Object%20Reference) (OtherComp :type Primitive%20Component%20Object%20Reference) (OtherBodyIndex :type Integer))
  (bind _ratchet (Variables|Default|GetRatchet))
  (if (== OtherActor _ratchet)
    (Variables|Default|SetShould%20trace%20for%20Ground false)
    (Variables|/Game/RatchetAndClank/Blueprints/Actors/Characters/Pawns/Ratchet.Ratchet_C|SetWalkOnWater _ratchet false)))

(event Custom|UnderNeathWater
  (bind _ratchet (Variables|Default|GetRatchet))
  (bind _ratchet_2 (Variables|Default|GetRatchet))
  (bind _charactermovement (Variables|/Script/Engine.Character|GetCharacterMovement _ratchet_2))
  (Utilities|FlowControl|Sequence
    (:then_0
      (CallFunction|StopBuoyancy)
      (Class|MovementComponent|SetPlaneConstraintEnabled _charactermovement false)
      (Pawn|Components|CharacterMovement|SetMovementMode _charactermovement "MOVE_Flying" 0)
      (Variables|/Game/RatchetAndClank/Blueprints/Actors/Characters/Pawns/Ratchet.Ratchet_C|SetSwimmingStates _ratchet_2 "NewEnumerator2")
      (Collision|SetCollisionEnabled (Variables|BP_Water_C|GetBox (Variables|/Game/RatchetAndClank/Blueprints/Actors/Characters/Pawns/Ratchet.Ratchet_C|GetWaterPLane (Variables|Default|GetRatchet))) "NoCollision")
      (Audio|PlaySoundatLocation "/Game/RatchetAndClank/Sounds/SFX/RC1Sfx/EnterWater_Cue.EnterWater_Cue" (Transformation|GetActorLocation (Variables|Default|GetRatchet)) "0, 0, 0" 1.0 1.0 0.0 0 0 0))
    (:then_1
      (bind _newtrack_0 (Timeline|Timeline_0 PlayFromStart)
        (:Update
          (Variables|/Script/Engine.MovementComponent|SetVelocity _charactermovement (* (Transformation|GetActorUpVector _ratchet) (* -5e+02 _newtrack_0)))
          (Variables|/Game/RatchetAndClank/Blueprints/Actors/Characters/Pawns/Ratchet.Ratchet_C|SetCapsuleX _ratchet -89.0))
        (:Finished
          (Variables|/Game/RatchetAndClank/Blueprints/Actors/Characters/Pawns/Ratchet.Ratchet_C|SetCapsuleX _ratchet 0.0))))))

(event Custom|Stop%20Buoyancy
  (bind _ratchet (Variables|Default|GetRatchet))
  (bind _returnvalue (Transformation|GetActorLocation _ratchet))
  (Variables|/Game/RatchetAndClank/Blueprints/Actors/Characters/Pawns/Ratchet.Ratchet_C|SetCan't%20Move _ratchet false)
  (bind _newtrack_0 (Timeline|Bouyancy Stop)
    (:Update
      (Transformation|SetActorLocation _ratchet (Math|Vector|MakeVector (.x _returnvalue) (.y _returnvalue) (+ _newtrack_0 (.z _returnvalue))) false false))
    (:Finished
      (Transformation|SetActorLocation _ratchet (Math|Vector|MakeVector (.x _returnvalue) (.y _returnvalue) (+ (.z (Transformation|GetActorLocation (Variables|/Game/RatchetAndClank/Blueprints/Actors/Characters/Pawns/Ratchet.Ratchet_C|GetWaterPLane (Variables|Default|GetRatchet)))) -2e+01)) false false))))

(event Custom|Getout%20of%20water
  (bind _ratchet (Variables|Default|GetRatchet))
  (bind _charactermovement (Variables|/Script/Engine.Character|GetCharacterMovement _ratchet))
  (Variables|/Game/RatchetAndClank/Blueprints/Actors/Characters/Pawns/Ratchet.Ratchet_C|SetSwimmingStates _ratchet "NewEnumerator0")
  (Variables|/Game/RatchetAndClank/Blueprints/Actors/Characters/Pawns/Ratchet.Ratchet_C|SetSwimming _ratchet false)
  (Rendering|SetActorHiddenInGame (Variables|/Game/RatchetAndClank/Blueprints/Actors/Characters/Pawns/Ratchet.Ratchet_C|GetCurrentWeapon _ratchet) false)
  (Variables|/Script/Engine.CharacterMovementComponent|SetMaxWalkSpeed _charactermovement 9e+02)
  (Collision|SetCollisionEnabled (Variables|BP_Water_C|GetBox (Variables|/Game/RatchetAndClank/Blueprints/Actors/Characters/Pawns/Ratchet.Ratchet_C|GetWaterPLane (Variables|Default|GetRatchet))) "QueryOnly")
  (Variables|/Script/Engine.CharacterMovementComponent|SetBrakingDecelerationFalling _charactermovement 5e+02)
  (Variables|/Script/Engine.CharacterMovementComponent|SetFallingLateralFriction _charactermovement 5.0)
  (Variables|/Script/Engine.PostProcessComponent|SetbEnabled (Variables|Default|Getpost) false)
  (Class|MovementComponent|SetPlaneConstraintEnabled (Variables|/Script/Engine.Character|GetCharacterMovement _ratchet) false))

(event Custom|Is%20Not%20swimmable
  (Variables|Default|SetIs%20Swimmable? false)
  (Variables|/Game/RatchetAndClank/Blueprints/Actors/Characters/Pawns/Ratchet.Ratchet_C|SetWalkOnWater (Variables|Default|GetRatchet) true))

(event Custom|Is%20now%20swimmable
  (Variables|Default|SetIs%20Swimmable? true)
  (Variables|/Game/RatchetAndClank/Blueprints/Actors/Characters/Pawns/Ratchet.Ratchet_C|SetWalkOnWater (Variables|Default|GetRatchet) false))

(event EventBeginPlay
  (bind _asratchet (Utilities|Casting|CastToRatchet (Game|GetPlayerCharacter 0)))
  (Variables|Default|SetRatchet _asratchet))

(event EventTick
  (params (DeltaSeconds :type Float%20%28single-precision%29))
  (bind _ratchet (Variables|Default|GetRatchet))
  (bind _post (Variables|Default|Getpost))
  (bind _waterplane (Variables|/Game/RatchetAndClank/Blueprints/Actors/Characters/Pawns/Ratchet.Ratchet_C|GetWaterPLane _ratchet))
  (bind _swimming (Variables|/Game/RatchetAndClank/Blueprints/Actors/Characters/Pawns/Ratchet.Ratchet_C|GetSwimming _ratchet))
  (bind _returnvalue (Transformation|GetActorLocation _waterplane))
  (Variables|Default|SetDelta DeltaSeconds)
  (Utilities|FlowControl|Sequence
    (:then_0
      (Utilities|IsValid _waterplane
        (:Is%20Valid
          (if _swimming
            (if (and (> (.z (Transformation|GetActorLocation _ratchet)) (.z _returnvalue)) (Utilities|Enum|Equal(Enum) (Variables|/Game/RatchetAndClank/Blueprints/Actors/Characters/Pawns/Ratchet.Ratchet_C|GetSwimmingStates (Variables|Default|GetRatchet)) "NewEnumerator2"))
              (Utilities|FlowControl|DoOnce false :!label _label
                (:Completed
                  (CallFunction|AboveWatr)))
              (else
                (goto _label Reset)))))))
    (:then_1
      (Utilities|IsValid _waterplane
        (:Is%20Valid
          (if _swimming
            (if (> (.z (Transformation|GetWorldLocation (Variables|/Script/RatchetAndClankTuts.RatchetAndClankTutsCharacter|GetFollowCamera _ratchet))) (.z _returnvalue))
              (Utilities|IsValid _post
                (:Is%20Valid
                  (Variables|/Script/Engine.PostProcessComponent|SetbEnabled _post false)))
              (else
                (Utilities|IsValid _post
                  (:Is%20Valid
                    (Variables|/Script/Engine.PostProcessComponent|SetbEnabled _post true)))))))))))

(fn ConstructionScript)

(event Custom|Above%20Watr
  (bind _ratchet (Variables|Default|GetRatchet))
  (bind _post (Variables|Default|Getpost))
  (bind _returnvalue (Transformation|GetActorLocation _ratchet))
  (bind _charactermovement (Variables|/Script/Engine.Character|GetCharacterMovement _ratchet))
  (Variables|/Game/RatchetAndClank/Blueprints/Actors/Characters/Pawns/Ratchet.Ratchet_C|SetCapsuleX _ratchet 0.0)
  (Variables|/Game/RatchetAndClank/Blueprints/Actors/Characters/Pawns/Ratchet.Ratchet_C|SetSwimmingStates _ratchet "NewEnumerator1")
  (Variables|/Script/Engine.CharacterMovementComponent|SetBrakingDecelerationFalling _charactermovement 2e+02)
  (Variables|/Script/Engine.CharacterMovementComponent|SetFallingLateralFriction _charactermovement 1.0)
  (Pawn|Components|CharacterMovement|SetMovementMode _charactermovement "MOVE_Falling" 0)
  (Transformation|SetActorLocation _ratchet (Math|Vector|MakeVector (.x _returnvalue) (.y _returnvalue) (+ (.z (Transformation|GetActorLocation (Variables|/Game/RatchetAndClank/Blueprints/Actors/Characters/Pawns/Ratchet.Ratchet_C|GetWaterPLane _ratchet))) -2e+01)) false false)
  (Utilities|IsValid _post
    (:Is%20Valid
      (Variables|/Script/Engine.PostProcessComponent|SetbEnabled _post false)
      (return))))
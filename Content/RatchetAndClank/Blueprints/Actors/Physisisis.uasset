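; Physics sphere actor that appears to support Ratchet's grapple, with mass scale set from a character's movement mass through a custom event.
; Each tick it clamps the sphere's linear velocity per axis and adds downward acceleration, stronger when Ratchet is level with or above his grapple target than when below.
; It also prints a normalized dot product of its velocity and Ratchet's forward vector for debugging.
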(event Custom|Mass%20Update%20on%20Spawn
  (params (ThirdPersonCharacter :type Ratchet%20Object%20Reference))
  (Class|PrimitiveComponent|SetMassScale (Variables|Default|GetSphere) "None" (Variables|/Script/Engine.CharacterMovementComponent|GetMass (Variables|/Script/Engine.Character|GetCharacterMovement ThirdPersonCharacter))))

(event EventBeginPlay
  (bind _asratchet (Utilities|Casting|CastToRatchet (Game|GetPlayerCharacter 0)))
  (Variables|Default|SetNewVar_0 _asratchet))

(event EventTick
  (params (DeltaSeconds :type Float%20%28single-precision%29))
  (bind _sphere (Variables|Default|GetSphere))
  (bind _sphere_2 (Variables|Default|GetSphere))
  (bind _newvar_0 (Variables|Default|GetNewVar_0))
  (Utilities|FlowControl|Sequence
    (:then_0
      (bind _returnvalue (Physics|GetPhysicsLinearVelocity _sphere_2 "None"))
      (Class|PrimitiveComponent|SetAllPhysicsLinearVelocity _sphere_2 (Math|Vector|MakeVector (Math|Float|Clamp(Float) (.x _returnvalue) -3.5e+03 3.5e+03) (Math|Float|Clamp(Float) (.y _returnvalue) -3.5e+03 3.5e+03) (Math|Float|Clamp(Float) (.z _returnvalue) -3e+03 3e+03)) false)
      (Math|Float|CompareFloat (.z (Transformation|GetActorLocation _newvar_0)) (.z (Transformation|GetActorLocation (Variables|/Game/RatchetAndClank/Blueprints/Actors/Characters/Pawns/Ratchet.Ratchet_C|GetGrapple%20Target _newvar_0)))
        (:>
          (Physics|AddForce _sphere "0.0,0.0,-6000.000000" "None" true :!label _label))
        (:==
          (goto _label))
        (:<
          (Physics|AddForce _sphere "0.0,0.0,-3000.0" "None" true))))
    (:then_1
      (Development|PrintString (Utilities|String|ToString(Float) (Math|Float|NormalizetoRange (Math|Float|Clamp(Float) (Math|Vector|DotProduct (Transformation|GetVelocity) (Transformation|GetActorForwardVector (Variables|Default|GetNewVar_0))) -1e+03 1e+03) -1e+03 1e+03)) true true "(R=0.000000,G=0.660000,B=1.000000,A=1.000000)" 0.0))))

(fn ConstructionScript)
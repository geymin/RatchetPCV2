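; Temporary bolt dispenser actor that turns a bolt amount passed to Init into pickup actors, then destroys itself.
; A delayed loop spawns one bolt per pass, choosing gear, washer, nut or standard by the remaining amount and subtracting its value.
; Gears require half the remainder to exceed their value, leaving more for smaller bolts.
; Spawn transforms come from RandomTransformBolts_2, whose random offset-and-rotation node appears unconnected.
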(event Custom|Init
  (params (boltsToSpawn :type Integer))
  (bind _randomtransform (|RandomTransformBolts_2))
  (if (== boltsToSpawn 0)
    _
    (else
      (Variables|Default|SetboltsToSpawn boltsToSpawn)
      (if (> (/ (Variables|Default|GetboltsToSpawn) 2) 50) :!label _label
        (Game|SpawnActorfromClass "/Game/RatchetAndClank/Blueprints/Actors/Bolts/BP_Bolt/GearsBolt.GearsBolt_C" _randomtransform "Undefined" 0 0)
        (Variables|Default|SetboltsToSpawn (- (Variables|Default|GetboltsToSpawn) 50))
        (elif (> (Variables|Default|GetboltsToSpawn) 20)
          (Game|SpawnActorfromClass "/Game/RatchetAndClank/Blueprints/Actors/Bolts/BP_Bolt/WasherBolt.WasherBolt_C" _randomtransform "Undefined" 0 0)
          (Variables|Default|SetboltsToSpawn (- (Variables|Default|GetboltsToSpawn) 20))
          (elif (> (Variables|Default|GetboltsToSpawn) 5)
            (Game|SpawnActorfromClass "/Game/RatchetAndClank/Blueprints/Actors/Bolts/BP_Bolt/NutBolt.NutBolt_C" _randomtransform "Undefined" 0 0)
            (Variables|Default|SetboltsToSpawn (- (Variables|Default|GetboltsToSpawn) 5))
            (else
              (Game|SpawnActorfromClass "/Game/RatchetAndClank/Blueprints/Actors/Bolts/BP_Bolt/StandardBolt.StandardBolt_C" _randomtransform "Undefined" 0 0)
              (Variables|Default|SetboltsToSpawn (- (Variables|Default|GetboltsToSpawn) 1))))))
      (Utilities|FlowControl|Delay 0.0001)
      (if (not (<= (Variables|Default|GetboltsToSpawn) 0))
        (goto _label)
        (else
          _))))
  (Actor|DestroyActor))

(event EventBeginPlay)

(event Collision|EventActorBeginOverlap
  (params (OtherActor :type Actor%20Object%20Reference)))

(event EventTick
  (params (DeltaSeconds :type Float%20%28single-precision%29)))

(fn ConstructionScript)
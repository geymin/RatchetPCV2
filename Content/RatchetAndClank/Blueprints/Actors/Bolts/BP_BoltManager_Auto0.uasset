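; BP_BoltManager_Auto0 is a level bolt manager that automatically spreads the level's standard bolt budget across crates.
; All work runs in the construction script, which first sends itself to the game mode with zero reserve bolts.
; It gathers unique crates from the Crates arrays of placed actors, then gives each an equal share plus a deviation percent.
; A text render shows the crate count and average bolts per crate.
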(event Collision|EventActorBeginOverlap
  (params (OtherActor :type Actor%20Object%20Reference)))

(event EventTick
  (params (DeltaSeconds :type Float%20%28single-precision%29)))

(fn ConstructionScript
  (Class|Object|ISendReserveBolts(Message) (Game|GetGameMode) self)
  (bind _outactors (Actor|GetAllActorsOfClass 0))
  (Variables|Default|SetArrayOfCrates 0 _outactors)
  (bind _outactors_2 (Actor|GetAllActorsOfClass 0))
  (for _array_element _outactors_2
    (for _array_element_2 (Variables|Default|GetCrates _array_element)
      (Utilities|Array|AddUnique (.ArrayOfCrates (Variables|Default|GetArrayOfCrates)) _array_element_2)))
  (for _array_element_3 (.ArrayOfCrates (Variables|Default|GetArrayOfCrates))
    (CallFunction|SetBoltAmount _array_element_3 (/ (Variables|Default|GetStandardBoltsInLevel) (Utilities|Array|Length (.ArrayOfCrates (Variables|Default|GetArrayOfCrates)))) (Variables|Default|GetBoltDeviationPercent))
    (Rendering|Components|TextRender|SetText (Variables|Default|GetTextRender) (Utilities|Text|ToText(String) (Utilities|String|Append (Utilities|String|ToString(Integer) (Utilities|Array|Length (.ArrayOfCrates (Variables|Default|GetArrayOfCrates)))) "-Crates " (Utilities|String|ToString(Integer) (/ (Variables|Default|GetStandardBoltsInLevel) (Utilities|Array|Length (.ArrayOfCrates (Variables|Default|GetArrayOfCrates))))) "-Bolts per Crate (average)")))))
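; BP_SlamButton is a single-use button actor that sinks when its ActivatedButton event is triggered.
; If CanUse is set, the event plays a press sound at the actor and clears the flag, with no reset in this graph.
; MoveComponentTo then interpolates AvioPackButton over InterpTime to a relative Z of negated ValueZ, keeping its X, Y and rotation.
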(event Custom|Activated%20Button
  (bind _aviopackbutton (Variables|Default|GetAvioPackButton))
  (bind _relativelocation (Variables|/Script/Engine.SceneComponent|GetRelativeLocation _aviopackbutton))
  (if (Variables|Default|GetCan%20Use)
    (Audio|PlaySoundatLocation "/Game/RatchetAndClank/Sounds/SFX/RC1Sfx/PressButton_Cue.PressButton_Cue" (Transformation|GetActorLocation) "0, 0, 0" 1.0 1.0 0.0 0 0 0)
    (Variables|Default|SetCan%20Use false)
    (Components|MoveComponentTo _aviopackbutton (Math|Vector|MakeVector (.x _relativelocation) (.y _relativelocation) (* (Variables|Default|GetValueZ) -1.0)) (Variables|/Script/Engine.SceneComponent|GetRelativeRotation _aviopackbutton) false false (Variables|Default|GetInterp%20Time) false)))

(event EventBeginPlay)

(event EventTick
  (params (DeltaSeconds :type Float%20%28single-precision%29)))

(fn ConstructionScript)
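; A mover actor that shuttles or loops its root between its starting transform and a destination given as a location and rotation offset.
; BeginPlay resolves both transforms and starts in the chosen direction, with the Motion timeline driving the transform lerp at a play rate set from Speed in the construction script.
; At each end it either destroys itself or pauses, then reverses if PingPong is on or restarts the same direction if not.
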(event Custom|GoBack
  (bind _pause (Variables|Default|GetPause))
  (bind _pingpong_ (Variables|Default|GetPingPong?))
  (bind (_direction _progress) (Timeline|Motion ReverseFromEnd)
    (:Update
      (Transformation|SetRelativeTransform (Variables|Default|GetDefaultSceneRoot) (Math|Transform|Lerp(Transform) (Variables|Default|GetStartingPosition) (Variables|Default|GetDestinationPosition) _progress) false false))
    (:Finished
      (if (Variables|Default|GetDestroyOnFinish?)
        (Actor|DestroyActor)
        (else
          (switch Utilities|FlowControl|Switch|SwitchonETimelineDirection _direction
            (:Forward
              (Utilities|FlowControl|Delay _pause)
              (if _pingpong_
                (CallFunction|GoBack :!label _label)
                (else
                  (CallFunction|GoForward :!label _label_2))))
            (:Backward
              (Utilities|FlowControl|Delay _pause)
              (if _pingpong_
                (goto _label_2)
                (else
                  (goto _label))))))))))

(event Custom|GoForward
  (bind _pause (Variables|Default|GetPause))
  (bind _pingpong_ (Variables|Default|GetPingPong?))
  (bind (_direction _progress) (Timeline|Motion PlayFromStart)
    (:Update
      (Transformation|SetRelativeTransform (Variables|Default|GetDefaultSceneRoot) (Math|Transform|Lerp(Transform) (Variables|Default|GetStartingPosition) (Variables|Default|GetDestinationPosition) _progress) false false))
    (:Finished
      (if (Variables|Default|GetDestroyOnFinish?)
        (Actor|DestroyActor)
        (else
          (switch Utilities|FlowControl|Switch|SwitchonETimelineDirection _direction
            (:Forward
              (Utilities|FlowControl|Delay _pause)
              (if _pingpong_
                (CallFunction|GoBack :!label _label)
                (else
                  (CallFunction|GoForward :!label _label_2))))
            (:Backward
              (Utilities|FlowControl|Delay _pause)
              (if _pingpong_
                (goto _label_2)
                (else
                  (goto _label))))))))))

(event Collision|EventActorBeginOverlap
  (params (OtherActor :type Actor%20Object%20Reference)))

(event EventBeginPlay
  (bind _defaultsceneroot (Variables|Default|GetDefaultSceneRoot))
  (bind _returnvalue (Transformation|GetWorldTransform _defaultsceneroot))
  (bind (_location _rotation) (Math|Transform|BreakTransform _returnvalue))
  (bind (_roll _pitch _yaw) (Math|Rotator|BreakRotator _rotation))
  ;[1 1 1] BeginPlay
  (Variables|Default|SetStartingPosition _returnvalue)
  (Variables|Default|SetDestinationPosition (Math|Transform|MakeTransform (+ _location (.Location (Math|Transform|BreakTransform (Variables|Default|GetDestinationPosition)))) (Math|Rotator|MakeRotator (+ _roll (.Roll (Math|Rotator|BreakRotator (.Rotation (Math|Transform|BreakTransform (Variables|Default|GetDestinationPosition)))))) (+ _pitch (.Pitch (Math|Rotator|BreakRotator (.Rotation (Math|Transform|BreakTransform (Variables|Default|GetDestinationPosition)))))) (+ _yaw (.Yaw (Math|Rotator|BreakRotator (.Rotation (Math|Transform|BreakTransform (Variables|Default|GetDestinationPosition))))))) (.Scale (Math|Transform|BreakTransform (Variables|Default|GetDestinationPosition)))))
  (if (Variables|Default|GetStartForward?)
    (CallFunction|GoForward)
    (else
      (CallFunction|GoBack))))

(fn ConstructionScript
  (Components|Timeline|SetPlayRate (Variables|Default|GetMotion) (Variables|Default|GetSpeed)))
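; Bolt crank interactable from Ratchet & Clank that Ratchet turns by walking it around until a target amount is reached.
; An overlap sphere flags availability, and an arrow tracks Ratchet to choose the grab side.
; SetRatchettoLocation blends to the crank camera and moves him to a spawned stance component attached to the bolt.
; Tick turns smoothed stick input into bolt rotation and progress, calling Exit to release him at the target.
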(event OnComponentBeginOverlap(Sphere)
  (params (OverlappedComponent :type Primitive%20Component%20Object%20Reference) (OtherActor :type Actor%20Object%20Reference) (OtherComp :type Primitive%20Component%20Object%20Reference) (OtherBodyIndex :type Integer) (bFromSweep :type Boolean) (SweepResult :type Hit%20Result%20Structure%20%28by%20ref%29))
  (bind _ratchet (Variables|Default|GetRatchet))
  (if (Math|Boolean|ANDBoolean (== OtherActor _ratchet) (not (Variables|/Game/RatchetAndClank/Blueprints/Actors/Characters/Pawns/Ratchet.Ratchet_C|GetAnimDoSecondSwing _ratchet)) (not (Variables|/Game/RatchetAndClank/Blueprints/Actors/Characters/Pawns/Ratchet.Ratchet_C|GetAnimDoThirdSwing _ratchet)))
    (Variables|/Game/RatchetAndClank/Blueprints/Actors/Characters/Pawns/Ratchet.Ratchet_C|SetCanBoltCrank _ratchet true)))

(event OnComponentEndOverlap(Sphere)
  (params (OverlappedComponent :type Primitive%20Component%20Object%20Reference) (OtherActor :type Actor%20Object%20Reference) (OtherComp :type Primitive%20Component%20Object%20Reference) (OtherBodyIndex :type Integer))
  (if (== OtherActor (Variables|Default|GetRatchet))
    (Variables|/Game/RatchetAndClank/Blueprints/Actors/Characters/Pawns/Ratchet.Ratchet_C|SetCanBoltCrank (Variables|Default|GetRatchet) false)))

(event Custom|Set%20Ratchet%20to%20Location
  (bind _arrow (Variables|Default|GetArrow))
  (bind _arrow_2 (Variables|Default|GetArrow))
  (bind _bolt (Variables|Default|GetBolt))
  (bind _ratchet (Variables|Default|GetRatchet))
  (bind _returnvalue (Transformation|GetWorldRotation _arrow))
  (bind _returnvalue_2 (Transformation|GetWorldLocation _arrow_2))
  (bind _returnvalue_3 (Math|Vector|GetForwardVector _returnvalue))
  (bind _returnvalue_4 (Math|Vector|GetRightVector _returnvalue))
  (bind (_x _y _z) (Math|Vector|BreakVector _returnvalue_2))
  (bind _returnvalue_5 (* _returnvalue_4 35.0))
  (bind _returnvalue_6 (Math|Conversions|RotationFromXVector _returnvalue_3))
  (bind _returnvalue_7 (* _returnvalue_3 2e+02))
  (bind _returnvalue_8 (+ _z 9e+01))
  (bind _returnvalue_9 (Math|Rotator|CombineRotators _returnvalue_6 "0,-90.000000, 0"))
  (bind _returnvalue_10 (+ _y (.y _returnvalue_7) (.y _returnvalue_5)))
  (bind _returnvalue_11 (+ _x (.x _returnvalue_7) (.x _returnvalue_5)))
  (bind _returnvalue_12 (Math|Vector|MakeVector _returnvalue_11 _returnvalue_10 _returnvalue_8))
  (Utilities|FlowControl|Sequence
    (:then_0
      (Game|Player|SetViewTargetwithBlend (Game|GetPlayerController _ratchet) (Variables|Default|GetCamera) 1.0 "VTBlend_Cubic" 1.0 true))
    (:then_1
      (bind _returnvalue_13 (AddComponent|AddStaticMeshComponent true (Math|Transform|MakeTransform _returnvalue_12 _returnvalue_9 "1,1,1")))
      (bind _output_get (Variables|Default|SetStance _returnvalue_13))
      (Variables|/Game/RatchetAndClank/Blueprints/Actors/Characters/Pawns/Ratchet.Ratchet_C|SetCan't%20Move _ratchet true)
      (Transformation|SetWorldRotation (Variables|Default|GetBolt) (Math|Rotator|MakeRotator 0.0 0.0 (.yaw (Math|Rotator|CombineRotators (Math|Rotator|FindLookatRotation (Transformation|GetWorldLocation (Variables|Default|GetArrow)) (Transformation|GetActorLocation (Variables|Default|GetRatchet))) "0, 0, 0"))) false false)
      (Components|MoveComponentTo (Variables|/Script/Engine.Character|GetCapsuleComponent (Variables|Default|GetRatchet)) _returnvalue_12 _returnvalue_9 true false 0.2 true)
      (Transformation|AttachComponentToComponent (Variables|Default|GetRatchet) _bolt "None" "KeepWorld" "KeepWorld" "KeepWorld" true)
      (Transformation|AttachComponentToComponent _output_get _bolt "None" "KeepWorld" "KeepWorld" "KeepWorld" true))))

(event Custom|Exit
  (bind _returnvalue (Game|GetPlayerController 0))
  (bind _ratchet (Variables|Default|GetRatchet))
  (Variables|/Game/RatchetAndClank/Blueprints/Actors/Characters/Pawns/Ratchet.Ratchet_C|SetCanBoltCrank _ratchet false)
  (Transformation|DetachFromActor _ratchet "KeepWorld" "KeepWorld" "KeepWorld")
  (Variables|/Game/RatchetAndClank/Blueprints/Actors/Characters/Pawns/Ratchet.Ratchet_C|SetIsBoltCraanking _ratchet false)
  (Variables|Default|SetPercentage 0.0)
  (Game|Player|SetViewTargetwithBlend _returnvalue (Variables|Default|GetRatchet) 1.0 "VTBlend_Cubic" 1.0 true)
  (Pawn|SetControlRotation _returnvalue (Transformation|GetActorRotation (Variables|Default|GetCamera)))
  (Variables|/Game/RatchetAndClank/Blueprints/Actors/Characters/Pawns/Ratchet.Ratchet_C|SetCan't%20Move (Variables|Default|GetRatchet) false)
  (Components|DestroyComponent (Variables|Default|GetStance)))

(event EventTick
  (params (DeltaSeconds :type Float%20%28single-precision%29))
  (bind _arrow (Variables|Default|GetArrow))
  (bind _ratchet (Variables|Default|GetRatchet))
  (bind _ratchet_2 (Variables|Default|GetRatchet))
  (bind _ratchet_3 (Variables|Default|GetRatchet))
  (bind _arrow_2 (Variables|Default|GetArrow))
  (bind _returnvalue (Transformation|GetWorldRotation _arrow))
  (bind _returnvalue_2 (Transformation|GetWorldLocation _arrow_2))
  (bind _returnvalue_3 (Transformation|GetActorLocation _ratchet_3))
  (bind _axisright (Variables|/Game/RatchetAndClank/Blueprints/Actors/Characters/Pawns/Ratchet.Ratchet_C|GetAxisRight _ratchet_2))
  (bind _axisforward (Variables|/Game/RatchetAndClank/Blueprints/Actors/Characters/Pawns/Ratchet.Ratchet_C|GetAxisForward _ratchet_2))
  (bind _returnvalue_4 (Math|Float|Absolute(Float) _axisright))
  (bind _returnvalue_5 (Math|Float|Absolute(Float) _axisforward))
  (bind _returnvalue_6 (+ _returnvalue_5 _returnvalue_4))
  (Variables|Default|SetDelta DeltaSeconds)
  (Utilities|FlowControl|Sequence
    (:then_0
      (if (Variables|/Game/RatchetAndClank/Blueprints/Actors/Characters/Pawns/Ratchet.Ratchet_C|GetIsBoltCraanking (Variables|Default|GetRatchet))
        (Transformation|SetActorRotation _ratchet (Math|Rotator|CombineRotators (Transformation|GetWorldRotation (Variables|Default|GetStance)) "0,13.000000, 0"))
        (Transformation|SetActorLocation _ratchet (Transformation|GetWorldLocation (Variables|Default|GetStance)) false false)
        (bind _output_get (Variables|Default|SetRunRate (Math|Float|Absolute(Float) (.Yaw (Math|Rotator|BreakRotator (* "0.000000,175.000000, 0" (* (Math|Float|Clamp(Float) (Variables|Default|GetForward%20Axis)) -1.0 (Variables|Default|GetDelta))))))))
        (Transformation|AddLocalRotation (Variables|Default|GetBolt) (* "0.000000,175.000000, 0" (* (Math|Float|Clamp(Float) (Variables|Default|GetForward%20Axis)) -1.0 (Variables|Default|GetDelta))) false false)
        (bind _output_get_2 (Variables|Default|SetPercentage (+ (Variables|Default|GetPercentage) (Math|Float|Clamp(Float) (Math|Float|Absolute(Float) _output_get) 0.0 0.1))))
        (if (>= _output_get_2 (Variables|Default|GetAmount%20to%20Reach))
          (CallFunction|Exit))
        (else
          (Transformation|SetWorldRotation _arrow (Math|Rotator|MakeRotator (.roll _returnvalue) (.pitch _returnvalue) (.yaw (Math|Rotator|FindLookatRotation (Math|Vector|MakeVector (.x _returnvalue_2) (.y _returnvalue_2) (.z _returnvalue_2)) (Math|Vector|MakeVector (.x _returnvalue_3) (.y _returnvalue_3) (.z _returnvalue_3))))) false false))))
    (:then_1
      (Variables|Default|SetForward%20Axis (Math|Interpolation|FInterpTo (Variables|Default|GetForward%20Axis) _returnvalue_6 (Variables|Default|GetDelta) (Math|Float|SelectFloat 5.0 1e+01 (> _returnvalue_6 0.0)))))))

(event EventBeginPlay
  (bind _asratchet (Utilities|Casting|CastToRatchet (Game|GetPlayerCharacter 0)))
  (bind _output_get (Variables|Default|SetRatchet _asratchet))
  (Variables|/Game/RatchetAndClank/Blueprints/Actors/Characters/Pawns/Ratchet.Ratchet_C|SetBoltCrank _output_get self))

(fn ConstructionScript)
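; Breakable Ratchet & Clank bolt crate that hides and plays a break sound when damaged.
; SetBoltAmount randomizes its bolt count, but bolt and debris spawning are unwired, as is the self-destroy step.
; On near-upright hits from stationary non-player actors, it traces down, snaps to the surface and disables physics.
; When destroyed, it traces upward and wakes physics on objects above with a downward impulse, so stacks fall.
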(event Custom|SetBoltAmount
  (params (BoltsInCrate :type Integer) (BoltDeviation :type Float%20%28single-precision%29))
  ;[1 1 1] SetBoltAmount
  (Variables|BoltValues|SetRandomBoltDeviation BoltDeviation)
  (if (not (Variables|BoltValues|GetoverrideBoltManager?))
    (Variables|BoltValues|SetBolts%20to%20Spawn (Math|Float|Truncate (* BoltsInCrate (Math|Random|RandomFloatinRange (- 1.0 (Variables|BoltValues|GetRandomBoltDeviation)) (+ (Variables|BoltValues|GetRandomBoltDeviation) 1.0)))))))

(event EventDestroyed
  (bind _returnvalue (Transformation|GetActorLocation))
  (bind _returnvalue_2 (Transformation|GetActorUpVector))
  ;[1 1 1] Physics
  (bind _outhits (Class|KismetSystemLibrary|LineTraceMultiforObjects (+ _returnvalue (* _returnvalue_2 8e+01)) (+ _returnvalue (* _returnvalue_2 5e+03)) (Utilities|Array|MakeArray "ObjectTypeQuery9") false 0 "None" true "(R=1.000000,G=0.000000,B=0.000000,A=1.000000)" "(R=0.000000,G=1.000000,B=0.000000,A=1.000000)" 2e+01))
  (for _array_element _outhits
    (if (.bBlockingHit (Collision|BreakHitResult _array_element))
      (Physics|SetSimulatePhysics (.HitComponent (Collision|BreakHitResult _array_element)) true)
      (Physics|AddImpulse (.HitComponent (Collision|BreakHitResult _array_element)) "0, 0,-250.000000" "None" true))))

(event Collision|EventHit
  (params (MyComp :type Primitive%20Component%20Object%20Reference) (Other :type Actor%20Object%20Reference) (OtherComp :type Primitive%20Component%20Object%20Reference) (bSelfMoved :type Boolean) (HitLocation :type Vector :default "0, 0, 0") (HitNormal :type Vector :default "0, 0, 0") (NormalImpulse :type Vector :default "0, 0, 0") (Hit :type Hit%20Result%20Structure%20%28by%20ref%29))
  (bind _returnvalue (Transformation|GetActorLocation))
  ;[1 1 1] EventHit
  (Utilities|IsValid Other
    (:Is%20Valid
      (if (Math|Boolean|ANDBoolean (!= Other (Variables|Default|GetRatchet)) (Math|Float|InRange(Float) (Class|KismetMathLibrary|DegAcos (Math|Vector|DotProduct HitNormal (Transformation|GetActorUpVector))) 0.0 31.0) (!= Other self) (== (Math|Vector|VectorLength (Transformation|GetVelocity Other)) 0.0))
        (bind _outhit (Collision|LineTraceByChannel (+ _returnvalue "0,0.000000,50.000000") (+ _returnvalue (* (Transformation|GetActorUpVector) -9e+01)) "TraceTypeQuery1" false 0 "None" true "(R=0.194129,G=1.000000,B=0.000000,A=1.000000)" "(R=0.000000,G=0.819498,B=1.000000,A=1.000000)" 2e+01))
        (if (.bblockinghit _outhit)
          (Transformation|SetActorLocation (.impactpoint _outhit) false false)
          (Physics|SetSimulatePhysics (Variables|Default|GetBoltcrate) false))))))

(event EventBeginPlay
  ;[1 1 1] BeginPlay
  (bind _asratchet (Utilities|Casting|CastToRatchet (Game|GetPlayerCharacter 0)))
  (Variables|Default|SetRatchet _asratchet))

(event Game|Damage|EventAnyDamage
  (params (Damage :type Float%20%28single-precision%29) (DamageType :type Damage%20Type%20Object%20Reference) (InstigatedBy :type Controller%20Object%20Reference) (DamageCauser :type Actor%20Object%20Reference))
  (bind _boltcrate (Variables|Default|GetBoltcrate))
  ;[1 1 1] DamageTaken
  (Utilities|IsValid _boltcrate
    (:Is%20Valid
      (Rendering|SetVisibility _boltcrate false true)
      (Utilities|FlowControl|DoOnce false
        (:Completed
          ;[1 1 1] SpawnBolts
          (Utilities|FlowControl|Sequence
            (:then_0
              (Audio|PlaySoundatLocation (Variables|Default|GetBox%20break%20Sound) (Transformation|GetActorLocation) "0, 0, 0" 1.0 1.0 0.0 0 0 0)
              (if (not (> (/ (Variables|BoltValues|GetBolts%20to%20Spawn) 2) 50))
                (if (not (> (Variables|BoltValues|GetBolts%20to%20Spawn) 20))
                  (if (> (Variables|BoltValues|GetBolts%20to%20Spawn) 5)
                    _))))
            (:then_1
              ;[1 1 1] Debris
              (for _index (range 0 (Math|Random|RandomIntegerinRange 2 3))
                _))))))))

(fn ConstructionScript)
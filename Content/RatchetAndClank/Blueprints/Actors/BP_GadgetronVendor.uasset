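; BP_GadgetronVendor is the Gadgetron vendor actor that Ratchet can open and close when nearby.
; Range overlap enables Ratchet's CanGadgetron and registers the vendor; Sphere end-overlap also sets that flag true rather than clearing it.
; PrintThis toggles the shop: opening fades to a vendor camera, hides and moves Ratchet, animates, then calls ShowGadgetron; closing animates and blends back.
; The construction script offsets the referenced camera from the vendor and aims it at the vendor.
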(event OnComponentEndOverlap(Sphere)
  (params (OverlappedComponent :type Primitive%20Component%20Object%20Reference) (OtherActor :type Actor%20Object%20Reference) (OtherComp :type Primitive%20Component%20Object%20Reference) (OtherBodyIndex :type Integer))
  (bind _asratchet (Utilities|Casting|CastToRatchet OtherActor))
  (Variables|/Game/RatchetAndClank/Blueprints/Actors/Characters/Pawns/Ratchet.Ratchet_C|SetCanGadgetron _asratchet true))

(event OnComponentBeginOverlap(Range)
  (params (OverlappedComponent :type Primitive%20Component%20Object%20Reference) (OtherActor :type Actor%20Object%20Reference) (OtherComp :type Primitive%20Component%20Object%20Reference) (OtherBodyIndex :type Integer) (bFromSweep :type Boolean) (SweepResult :type Hit%20Result%20Structure%20%28by%20ref%29))
  (bind _asratchet (Utilities|Casting|CastToRatchet OtherActor))
  (Variables|/Game/RatchetAndClank/Blueprints/Actors/Characters/Pawns/Ratchet.Ratchet_C|SetCanGadgetron _asratchet true)
  (Variables|/Game/RatchetAndClank/Blueprints/Actors/Characters/Pawns/Ratchet.Ratchet_C|SetGadgetronVendor _asratchet self))

(event EventPrintThis
  (bind _returnvalue (Game|GetPlayerCameraManager 0))
  (bind _ratchet (Variables|Default|GetRatchet))
  (if (Variables|Default|GetVendorOpen)
    (Variables|Default|SetVendorOpen false)
    (Components|Animation|PlayAnimation (Variables|Default|GetGADout) "/Game/RatchetAndClank/Meshes/Generic/GADout_Anim_Armature_EndedGadgetron.GADout_Anim_Armature_EndedGadgetron" false)
    (Utilities|FlowControl|Delay 1.0)
    (Transformation|SetActorLocation _ratchet (Transformation|GetWorldLocation (Variables|/Script/Engine.CameraActor|GetCameraComponent (Variables|Default|GetCamera))) false false)
    (Game|Player|SetViewTargetwithBlend (Game|GetPlayerController 0) _ratchet 1.0 "VTBlend_Cubic" 1.0 true)
    (Rendering|SetVisibility (Variables|/Script/Engine.Character|GetCapsuleComponent _ratchet) true true)
    (else
      (Variables|Default|SetVendorOpen true)
      (CameraFades|StartCameraFade :self _returnvalue :ToAlpha 1.0 :Duration 0.1 :bHoldWhenFinished true)
      (Utilities|FlowControl|Delay 0.3)
      (Transformation|SetActorLocation (Variables|Default|GetRatchet) (Transformation|GetWorldLocation (Variables|/Script/Engine.CameraActor|GetCameraComponent (Variables|Default|GetCamera))) false false)
      (Rendering|SetVisibility (Variables|/Script/Engine.Character|GetCapsuleComponent (Variables|Default|GetRatchet)) false true)
      (Game|Player|SetViewTargetwithBlend (Game|GetPlayerController 0) (Variables|Default|GetCamera) 0.0 "VTBlend_Linear" 0.0 false)
      (CameraFades|StartCameraFade :self _returnvalue :FromAlpha 1.0 :Duration 0.08)
      (Utilities|FlowControl|Delay 0.2)
      (Components|Animation|PlayAnimation (Variables|Default|GetGADout) "/Game/RatchetAndClank/Meshes/Generic/GADout_Anim_Armature_Entergadgetron.GADout_Anim_Armature_Entergadgetron" false)
      (Utilities|FlowControl|Delay 1.0)
      (Default|ShowGadgetron (Variables|Default|GetRatchet)))))

(event EventTick
  (params (DeltaSeconds :type Float%20%28single-precision%29))
  (|CallParentFunction DeltaSeconds))

(fn ConstructionScript
  (bind _camera (Variables|Default|GetCamera))
  (bind _defaultsceneroot (Variables|Default|GetDefaultSceneRoot))
  (bind _returnvalue (Transformation|GetWorldTransform _defaultsceneroot))
  (Transformation|SetActorTransform _camera (Math|Transform|MakeTransform (+ (.location _returnvalue) (Variables|Default|GetCameraLocation)) (Math|Rotator|FindLookatRotation (Transformation|GetActorLocation _camera) (+ (.location _returnvalue) "0, 0,200.000000")) (.scale _returnvalue)))
  (|CallParentFunction))
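; Rotator is a generic actor that continuously spins a configurable static mesh in the level.
; The construction script applies the exposed mesh, material for slot zero and world scale to its StaticMesh component.
; On Tick, it adds a relative rotation to the root component from separate per-axis rates multiplied by delta time, keeping the spin frame-rate independent.
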(event EventBeginPlay)

(event Collision|EventActorBeginOverlap
  (params (OtherActor :type Actor%20Object%20Reference)))

(event EventTick
  (params (DeltaSeconds :type Float%20%28single-precision%29))
  (Transformation|AddRelativeRotation (Variables|Default|GetDefaultSceneRoot) (Math|Rotator|MakeRotator (* DeltaSeconds (Variables|Rotation|GetRotationRateX)) (* (Variables|Rotation|GetRotationRateY) DeltaSeconds) (* (Variables|Rotation|GetRotationRateZ) DeltaSeconds)) false false))

(fn ConstructionScript
  (bind _staticmesh (Variables|Default|GetStaticMesh))
  (Utilities|IsValid _staticmesh
    (:Is%20Valid
      (Components|StaticMesh|SetStaticMesh _staticmesh (Variables|Mesh|GetMesh))
      (Rendering|Material|SetMaterial _staticmesh 0 (Variables|Mesh|GetMeshMaterial))
      (Transformation|SetWorldScale3D _staticmesh (Variables|Mesh|GetMeshScale)))))
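; CrateStack is a Ratchet & Clank actor that builds a grid of stacked crates from child actors.
; The construction script clamps the X, Y and Z counts to at most ten, then adds an evenly spaced child actor component per slot.
; It offsets the grid around the origin horizontally, builds it upward and records each spawned actor in a Crates array.
; The event graph has no gameplay logic.
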(event EventBeginPlay)

(event Collision|EventActorBeginOverlap
  (params (OtherActor :type Actor%20Object%20Reference)))

(event EventTick
  (params (DeltaSeconds :type Float%20%28single-precision%29)))

(fn ConstructionScript
  (bind _stacks__x_ (Variables|Default|GetStacks%20%28X%29))
  (bind _stacks__y_ (Variables|Default|GetStacks%20%28Y%29))
  (bind _returnvalue (- _stacks__y_ 1))
  (bind _returnvalue_2 (- _stacks__x_ 1))
  (Utilities|Array|Clear (Variables|Default|GetCrates))
  (CallFunction|CapCrates)
  (for _index (range 0 _returnvalue)
    (for _index_2 (range 0 _returnvalue_2)
      (for _index_3 (range 0 (- (Variables|Default|GetCratesPerStack%20%28Z%29) 1))
        (bind _returnvalue_3 (AddComponent|AddChildActorComponent false (Math|Transform|MakeTransform (Math|Vector|MakeVector (- (* _index_2 145.0) (* _returnvalue_2 8e+01)) (- (* _index 145.0) (* _returnvalue 8e+01)) (* _index_3 145.0)) "0, 0, 0" "1,1,1")))
        (Utilities|Array|AddUnique (Variables|Default|GetCrates) (Variables|/Script/Engine.ChildActorComponent|GetChildActor _returnvalue_3))))))

(fn CapCrates
  (if (> (Variables|Default|GetStacks%20%28X%29) 10)
    (Variables|Default|SetStacks%20%28X%29 10))
  (if (> (Variables|Default|GetStacks%20%28Y%29) 10)
    (Variables|Default|SetStacks%20%28Y%29 10))
  (if (> (Variables|Default|GetCratesPerStack%20%28Z%29) 10)
    (Variables|Default|SetCratesPerStack%20%28Z%29 10)))
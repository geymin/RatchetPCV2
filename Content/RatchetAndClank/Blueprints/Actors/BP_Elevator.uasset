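; BP_Elevator is an elevator actor that slides its mesh between bottom and top positions.
; Overlapping the top or bottom trigger calls it to that end, while the riding trigger toggles direction when Moving is false.
; A single timeline plays or reverses to lerp the location, then clears Moving and re-enables both call triggers.
; The construction script places those triggers at the endpoints and sets timeline play rate from Speed.
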(event OnComponentBeginOverlap(RidingTrigger)
  (params (OverlappedComponent :type Primitive%20Component%20Object%20Reference) (OtherActor :type Actor%20Object%20Reference) (OtherComp :type Primitive%20Component%20Object%20Reference) (OtherBodyIndex :type Integer) (bFromSweep :type Boolean) (SweepResult :type Hit%20Result%20Structure%20%28by%20ref%29))
  (if (not (Variables|Default|Getmoving))
    (Variables|Default|Setmoving true)
    (if (Variables|Default|Getascended)
      (Variables|Default|Setascended false)
      (bind _alpha (Timeline|AscendTimeline Reverse)
        (:Update
          (Transformation|SetRelativeLocation (Variables|Default|GetElevatorMesh) (Math|Vector|Lerp(Vector) (Variables|Default|GetBottomTransform) (Variables|Default|GetTopTransform) _alpha) false false))
        (:Finished
          (Variables|Default|Setmoving false)
          (Collision|SetCollisionEnabled (Variables|Default|GetBottomTrigger) "QueryOnly")))
      (else
        (Variables|Default|Setascended true)
        (Timeline|AscendTimeline Play)))))

(event OnComponentBeginOverlap(BottomTrigger)
  (params (OverlappedComponent :type Primitive%20Component%20Object%20Reference) (OtherActor :type Actor%20Object%20Reference) (OtherComp :type Primitive%20Component%20Object%20Reference) (OtherBodyIndex :type Integer) (bFromSweep :type Boolean) (SweepResult :type Hit%20Result%20Structure%20%28by%20ref%29))
  (Collision|SetCollisionEnabled (Variables|Default|GetBottomTrigger) "NoCollision")
  (Variables|Default|Setascended false)
  (bind _alpha (Timeline|AscendTimeline Reverse)
    (:Update
      (Transformation|SetRelativeLocation (Variables|Default|GetElevatorMesh) (Math|Vector|Lerp(Vector) (Variables|Default|GetBottomTransform) (Variables|Default|GetTopTransform) _alpha) false false))
    (:Finished
      (Variables|Default|Setmoving false)
      (Collision|SetCollisionEnabled (Variables|Default|GetBottomTrigger) "QueryOnly"))))

(event OnComponentBeginOverlap(TopTrigger)
  (params (OverlappedComponent :type Primitive%20Component%20Object%20Reference) (OtherActor :type Actor%20Object%20Reference) (OtherComp :type Primitive%20Component%20Object%20Reference) (OtherBodyIndex :type Integer) (bFromSweep :type Boolean) (SweepResult :type Hit%20Result%20Structure%20%28by%20ref%29))
  (Collision|SetCollisionEnabled (Variables|Default|GetTopTrigger) "NoCollision")
  (Variables|Default|Setascended true)
  (bind _alpha (Timeline|AscendTimeline Play)
    (:Update
      (Transformation|SetRelativeLocation (Variables|Default|GetElevatorMesh) (Math|Vector|Lerp(Vector) (Variables|Default|GetBottomTransform) (Variables|Default|GetTopTransform) _alpha) false false))
    (:Finished
      (Variables|Default|Setmoving false)
      (Collision|SetCollisionEnabled (Variables|Default|GetBottomTrigger) "QueryOnly"))))

(event EventBeginPlay)

(event Collision|EventActorBeginOverlap
  (params (OtherActor :type Actor%20Object%20Reference)))

(event EventTick
  (params (DeltaSeconds :type Float%20%28single-precision%29)))

(fn ConstructionScript
  (Transformation|SetRelativeLocation (Variables|Default|GetBottomTrigger) (Variables|Default|GetBottomTransform) false false)
  (Transformation|SetRelativeLocation (Variables|Default|GetTopTrigger) (Variables|Default|GetTopTransform) false false)
  (Components|Timeline|SetPlayRate (Variables|Default|GetAscendTimeline) (Variables|Default|GetSpeed)))
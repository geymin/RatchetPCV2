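; CheckpointManager is an actor that relays reached checkpoints to the player pawn for saving.
; On BeginPlay it gathers every Checkpoint actor in the level and initializes each with a reference to itself.
; When the ICheckpointReached event reports a checkpoint different from the last one, it prints the location, sends ISaveMessage with location and spawn transform to the pawn, and remembers that checkpoint.
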(event EventBeginPlay
  (bind _outactors (Actor|GetAllActorsOfClass "/Game/RatchetAndClank/Blueprints/SaveSystem/Checkpoint.Checkpoint_C"))
  (bind _output_get (Variables|Default|SetLevelCheckpoints _outactors))
  (for _array_element _output_get
    (Default|Init _array_element self)))

(event Collision|EventActorBeginOverlap
  (params (OtherActor :type Actor%20Object%20Reference)))

(event EventTick
  (params (DeltaSeconds :type Float%20%28single-precision%29)))

(event EventICheckpointReached
  (params (CheckpointHit :type %20Object%20Reference) (CheckpointLocation :type Text) (PlayerPawn :type Pawn%20Object%20Reference) (CheckpointSpawnPoint :type Transform))
  (if (!= CheckpointHit (Variables|Default|GetLastCheckpointHit))
    (Development|PrintText CheckpointLocation true true "(R=0.200309,G=1.000000,B=0.000000,A=1.000000)")
    (Class|ICheckpoint|ISave(Message) PlayerPawn CheckpointLocation CheckpointSpawnPoint)
    (Variables|Default|SetLastCheckpointHit CheckpointHit)))

(fn ConstructionScript)
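; Teleporter pad that sends Ratchet to its linked TelePlace with a scale-based warp effect.
; Sphere overlap gates the PrintThis event; a DoOnce blocks retriggering until the teleport finishes.
; It locks Ratchet's controls and uses a timeline to walk him onto the pad.
; Timelines then thin his mesh and animate the probe effect, move him, snap the camera to the exit's facing, and restore scale and controls.
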(event OnComponentBeginOverlap(Sphere)
  (params (OverlappedComponent :type Primitive%20Component%20Object%20Reference) (OtherActor :type Actor%20Object%20Reference) (OtherComp :type Primitive%20Component%20Object%20Reference) (OtherBodyIndex :type Integer) (bFromSweep :type Boolean) (SweepResult :type Hit%20Result%20Structure%20%28by%20ref%29))
  (if (== OtherActor (Variables|Default|GetRatchet))
    (Variables|Default|SetIs%20Enabled%20Teleporting? true)
    (Utilities|FlowControl|Gate true) ; enters at Open
  ))

(event OnComponentEndOverlap(Sphere)
  (params (OverlappedComponent :type Primitive%20Component%20Object%20Reference) (OtherActor :type Actor%20Object%20Reference) (OtherComp :type Primitive%20Component%20Object%20Reference) (OtherBodyIndex :type Integer))
  (if (== OtherActor (Variables|Default|GetRatchet))
    (Variables|Default|SetIs%20Enabled%20Teleporting? false)
    (Utilities|FlowControl|Gate true) ; enters at Close
  ))

(event Custom|Teleport%20Finished
  (Utilities|FlowControl|DoOnce false) ; enters at Reset
)

(event EventBeginPlay
  (|CallParentFunction)
  (bind _asratchet (Utilities|Casting|CastToRatchet (Game|GetPlayerCharacter 0)))
  (Variables|Default|SetRatchet _asratchet))

(event EventTick
  (params (DeltaSeconds :type Float%20%28single-precision%29))
  (|CallParentFunction DeltaSeconds))

(event EventPrintThis
  (Utilities|FlowControl|Gate true
    (:Exit
      (CallFunction|UndoHudShit)
      (Utilities|FlowControl|DoOnce false
        (:Completed
          (|WalktoSpot))))))

(fn ConstructionScript
  (|CallParentFunction))

(event Custom|Set%20scale%20part
  (bind _returnvalue (Transformation|GetActorLocation))
  (bind _ratchet (Variables|Default|GetRatchet))
  (bind _ratchet_2 (Variables|Default|GetRatchet))
  (bind _ratchet_3 (Variables|Default|GetRatchet))
  (bind _ratchet_4 (Variables|Default|GetRatchet))
  (bind _ratchet_5 (Variables|Default|GetRatchet))
  (bind _ratchet_6 (Variables|Default|GetRatchet))
  (bind _probe_effect (Variables|Default|GetProbe_Effect))
  (bind _teleplace (Variables|Default|GetTelePlace))
  (bind _ratchet_7 (Variables|Default|GetRatchet))
  (bind _ratchet_8 (Variables|Default|GetRatchet))
  (bind _teleporter (Variables|Default|GetTeleporter))
  (bind _returnvalue_2 (Transformation|GetActorLocation _ratchet_8))
  (bind _returnvalue_3 (Transformation|GetWorldLocation _teleporter))
  (bind _returnvalue_4 (Transformation|GetActorLocation _ratchet_3))
  (bind _mesh (Variables|/Script/Engine.Character|GetMesh _ratchet_4))
  (bind _face_this_direction (Variables|BP_Teleporter2_C|GetFace%20this%20direction _teleplace))
  (bind _cameraboom (Variables|/Script/RatchetAndClankTuts.RatchetAndClankTutsCharacter|GetCameraBoom _ratchet_6))
  (bind _returnvalue_5 (- _returnvalue_2 _returnvalue_3))
  (bind _returnvalue_6 (Math|Vector|GetUnitDirection(Vector) _returnvalue_4 _returnvalue))
  (bind _returnvalue_7 (Transformation|GetWorldRotation _face_this_direction))
  (bind _returnvalue_8 (Math|Vector|VectorLength (Math|Vector|MakeVector (.x _returnvalue_5) (.y _returnvalue_5) 0.0)))
  (bind _returnvalue_9 (Math|Vector|GetForwardVector _returnvalue_7))
  (bind _returnvalue_10 (Math|Conversions|RotationFromXVector _returnvalue_9))
  (Utilities|FlowControl|Sequence
    (:then_0
      (Variables|/Game/RatchetAndClank/Blueprints/Actors/Characters/Pawns/Ratchet.Ratchet_C|SetAxisForward _ratchet_5 0.0)
      (Timeline|Go%20to%20Where%20to%20Stand Stop
        (:Update
          (Pawn|Input|AddMovementInput _ratchet_3 (Math|Vector|MakeVector (.x _returnvalue_6) (.y _returnvalue_6) 0.0) 1.0 false)
          (Variables|/Game/RatchetAndClank/Blueprints/Actors/Characters/Pawns/Ratchet.Ratchet_C|SetTargetZ _ratchet_3 (Math|Rotator|MakeRotator 0.0 0.0 (.yaw (Math|Conversions|RotationFromXVector (Math|Vector|GetUnitDirection(Vector) _returnvalue_4 _returnvalue)))))
          (Variables|/Game/RatchetAndClank/Blueprints/Actors/Characters/Pawns/Ratchet.Ratchet_C|SetAxisForward _ratchet_3 (Math|Float|NormalizetoRange (Math|Float|Clamp(Float) _returnvalue_8 0.0 1.5e+02) 0.0 1.5e+02))
          (if (Math|Float|InRange(Float) _returnvalue_8 0.0 1.0)
            (CallFunction|SetScalePart)))))
    (:then_1
      (Audio|PlaySoundatLocation "/Game/RatchetAndClank/Sounds/SFX/RC1Sfx/TeleportStart.TeleportStart" (Transformation|GetActorLocation _ratchet_5) "0, 0, 0" 1.0 1.0 0.0 0 0 0)
      (Variables|Default|SetMesh%20Scale (Transformation|GetWorldScale (Variables|/Script/Engine.Character|GetMesh _ratchet_5)))
      (Variables|Default|SetProbe%20Scale (Transformation|GetWorldScale _probe_effect))
      (Utilities|FlowControl|Sequence
        (:then_0
          (Utilities|FlowControl|Delay 0.2)
          (bind (_direction _scale _probe_scale _newtrack_2) (Timeline|Timeline_0 PlayFromStart)
            (:Update
              (Variables|/Game/RatchetAndClank/Blueprints/Actors/Characters/Pawns/Ratchet.Ratchet_C|SetTargetZ _ratchet_7 (Math|Conversions|RotationFromXVector (Math|Vector|GetForwardVector (Transformation|GetWorldRotation (Variables|Default|GetFace%20this%20direction)))))
              (Transformation|SetWorldScale3D (Variables|/Script/Engine.Character|GetMesh _ratchet_7) (Math|Vector|Lerp(Vector) (Variables|Default|GetMesh%20Scale) (Math|Vector|MakeVector 0.0 0.0 (.Z (Math|Vector|BreakVector (Variables|Default|GetMesh%20Scale)))) _scale))
              (Transformation|SetWorldScale3D (Variables|Default|GetProbe_Effect) (Math|Vector|Lerp(Vector) (Variables|Default|GetProbe%20Scale) (Math|Vector|MakeVector 0.0 0.0 (Math|Float|Lerp (.Z (Math|Vector|BreakVector (Variables|Default|GetProbe%20Scale))) 15.0 _newtrack_2)) _probe_scale)))
            (:Finished
              (Utilities|FlowControl|Sequence
                (:then_0
                  (Variables|/Game/RatchetAndClank/Blueprints/Actors/Characters/Pawns/Ratchet.Ratchet_C|SetCamera%20Z%20Interpolation _ratchet_6 0.0)
                  (Transformation|SetActorLocation _ratchet_7 (+ (Transformation|GetActorLocation (Variables|Default|GetTelePlace)) "0, 0,90.000000") false false)
                  (Utilities|FlowControl|Delay 0.1)
                  (Audio|PlaySoundatLocation "/Game/RatchetAndClank/Sounds/SFX/RC1Sfx/TeleportEnd.TeleportEnd" (Transformation|GetActorLocation _ratchet_2) "0, 0, 0" 1.0 1.0 0.0 0 0 0)
                  (Transformation|SetActorRotation _ratchet_2 _returnvalue_10)
                  (Variables|/Game/RatchetAndClank/Blueprints/Actors/Characters/Pawns/Ratchet.Ratchet_C|SetTargetZ _ratchet_2 _returnvalue_10)
                  (Development|SetHiddeninGame (Variables|Default|GetProbe_Effect) true false)
                  (Development|SetHiddeninGame (Variables|BP_Teleporter2_C|GetProbe_Effect (Variables|Default|GetTelePlace)) false false)
                  (bind (_direction_2 _scale_2 _probe _z) (Timeline|Timeline_1 PlayFromStart)
                    (:Update
                      (Transformation|SetWorldScale3D _mesh (Math|Vector|Lerp(Vector) (Transformation|GetWorldScale _mesh) (Variables|Default|GetMesh%20Scale) _scale_2))
                      (Transformation|SetWorldScale3D (Variables|BP_Teleporter2_C|GetProbe_Effect (Variables|Default|GetTelePlace)) (Math|Vector|Lerp(Vector) (Transformation|GetWorldScale (Variables|Default|GetProbe_Effect)) (Math|Vector|MakeVector (+ (.x (Variables|Default|GetProbe%20Scale)) 7.0) (+ (.y (Variables|Default|GetProbe%20Scale)) 7.0) (Math|Float|Lerp 0.0 (.z (Variables|Default|GetProbe%20Scale)) _z)) _probe)))
                    (:Finished
                      (Variables|/Script/Engine.CharacterMovementComponent|SetMaxWalkSpeed (Variables|/Script/Engine.Character|GetCharacterMovement _ratchet) 9e+02)
                      (Variables|/Game/RatchetAndClank/Blueprints/Actors/Characters/Pawns/Ratchet.Ratchet_C|SetCan't%20Move _ratchet false)
                      (Variables|/Game/RatchetAndClank/Blueprints/Actors/Characters/Pawns/Ratchet.Ratchet_C|SetCan%20Jump _ratchet true)
                      (Variables|/Game/RatchetAndClank/Blueprints/Actors/Characters/Pawns/Ratchet.Ratchet_C|SetCanDoFirstSwing _ratchet true)
                      (Variables|/Game/RatchetAndClank/Blueprints/Actors/Characters/Pawns/Ratchet.Ratchet_C|SetCanDoSecondSwing _ratchet false)
                      (Variables|/Game/RatchetAndClank/Blueprints/Actors/Characters/Pawns/Ratchet.Ratchet_C|SetCanDoThirdSwing _ratchet false)
                      (Development|SetHiddeninGame (Variables|BP_Teleporter2_C|GetProbe_Effect (Variables|Default|GetTelePlace)) true false)
                      (Transformation|SetWorldScale3D (Variables|Default|GetProbe_Effect) (Variables|Default|GetProbe%20Scale))
                      (Transformation|SetWorldScale3D (Variables|BP_Teleporter2_C|GetProbe_Effect (Variables|Default|GetTelePlace)) (Variables|Default|GetProbe%20Scale))
                      (CallFunction|TeleportFinished)
                      (Variables|/Game/RatchetAndClank/Blueprints/Actors/Characters/Pawns/Ratchet.Ratchet_C|SetCamera%20Z%20Interpolation _ratchet 7.0))))
                (:then_1
                  (Variables|/Script/Engine.SpringArmComponent|SetbEnableCameraRotationLag _cameraboom false)
                  (Pawn|SetControlRotation (Game|GetPlayerController 0) _returnvalue_10)
                  (Utilities|FlowControl|Delay 0.06)
                  (Variables|/Script/Engine.SpringArmComponent|SetbEnableCameraRotationLag _cameraboom true))))))
        (:then_1
          (Utilities|FlowControl|Delay 0.6)
          (Development|SetHiddeninGame _probe_effect false false))))))
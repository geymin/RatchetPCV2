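; Base interactable actor for a Ratchet & Clank game that lets the player interact while inside its sphere trigger.
; On BeginPlay it caches the Ratchet pawn and creates a hidden InteractMessage widget in the viewport.
; Sphere overlaps set or clear Ratchet's CanInteract flag and Interact reference, fading the prompt in with empty text or out.
; A retriggerable delay matching the fade's length hides the widget afterward.
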(event OnComponentBeginOverlap(Sphere)
  (params (OverlappedComponent :type Primitive%20Component%20Object%20Reference) (OtherActor :type Actor%20Object%20Reference) (OtherComp :type Primitive%20Component%20Object%20Reference) (OtherBodyIndex :type Integer) (bFromSweep :type Boolean) (SweepResult :type Hit%20Result%20Structure%20%28by%20ref%29))
  (bind _ratchet (Variables|Default|GetRatchet))
  (if (== OtherActor _ratchet)
    (Variables|/Game/RatchetAndClank/Blueprints/Actors/Characters/Pawns/Ratchet.Ratchet_C|SetCanInteract _ratchet true)
    (Variables|/Game/RatchetAndClank/Blueprints/Actors/Characters/Pawns/Ratchet.Ratchet_C|SetInteract _ratchet self)
    (CallFunction|DoHUdShit)))

(event OnComponentEndOverlap(Sphere)
  (params (OverlappedComponent :type Primitive%20Component%20Object%20Reference) (OtherActor :type Actor%20Object%20Reference) (OtherComp :type Primitive%20Component%20Object%20Reference) (OtherBodyIndex :type Integer))
  (bind _ratchet (Variables|Default|GetRatchet))
  (if (== OtherActor (Variables|Default|GetRatchet))
    (Variables|/Game/RatchetAndClank/Blueprints/Actors/Characters/Pawns/Ratchet.Ratchet_C|SetCanInteract _ratchet false)
    (Variables|/Game/RatchetAndClank/Blueprints/Actors/Characters/Pawns/Ratchet.Ratchet_C|SetInteract _ratchet 0)
    (CallFunction|UndoHudShit)))

(event Custom|PrintThis)

(event Custom|UndoHudShit
  (bind _interactmessage (Variables|Default|GetInteractMessage))
  (Default|FadeOut _interactmessage)
  (Utilities|FlowControl|RetriggerableDelay (Class|WidgetAnimation|GetEndTime (Variables|/Game/RatchetAndClank/UI/InteractMessage.InteractMessage_C|GetFades _interactmessage)))
  (Widget|SetVisibility _interactmessage "Hidden"))

(event Custom|DoHUdShit
  (bind _interactmessage (Variables|Default|GetInteractMessage))
  (Widget|SetVisibility _interactmessage "Visible")
  (Default|FadeIN _interactmessage)
  (Default|UpdateText _interactmessage))

(event EventBeginPlay
  (bind _asratchet (Utilities|Casting|CastToRatchet (Game|Player|GetPlayerPawn 0)))
  (Variables|Default|SetRatchet _asratchet)
  (bind _returnvalue (UserInterface|CreateWidget "/Game/RatchetAndClank/UI/InteractMessage.InteractMessage_C"))
  (bind _output_get (Variables|Default|SetInteractMessage _returnvalue))
  (UserInterface|Viewport|AddtoViewport _output_get 0)
  (Widget|SetVisibility _output_get "Hidden"))

(event EventTick
  (params (DeltaSeconds :type Float%20%28single-precision%29)))

(fn ConstructionScript)